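; BP_Weapon is the character weapon, with hitscan primary fire, explosive projectile alternative fire and a gravity projectile special.
; Setup events pass per-mode fire data to inherited shot functions.
; Shot events play the owner's firing montage, then either draw a debug tracer and play random hit reactions on struck characters, or reveal the spawned projectile's mesh.
; Net-role macros and a debug sphere event are included, though the ownership switch sits only in dead code.
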(event EventEventonWeaponProjectileShot
  (params (Projectile :type Hi%20RS%20Projectile%20Object%20Reference))
  (bind _returnvalue (Components|GetOwner))
  (Utilities|IsValid _returnvalue
    (:Is%20Valid
      (bind _asbp_hi_rs_character (Utilities|Casting|CastToBP_HiRS_Character _returnvalue))
      (Animation|PlayAnimMontage _asbp_hi_rs_character "/Game/HiRS/Character/Animations/Montages/AM_Shooting_Hip.AM_Shooting_Hip" 1.0 "None")
      (Rendering|SetVisibility (Variables|/Script/HiRS.HiRS_Projectile|GetProjectileMesh Projectile) true true))))

(event EventEventonWeaponMomentalShot
  (params (HitResult :type Hit%20Result%20Structure))
  (bind _returnvalue (Components|GetOwner))
  (bind (_bblockinghit _binitialoverlap _time _location _impactpoint _normal _impactnormal _physmat _hitactor _hitcomponent _hitbonename _hititem _faceindex _tracestart _traceend) (Collision|BreakHitResult HitResult))
  (Utilities|FlowControl|Sequence
    (:then_0
      (Rendering|Debug|DrawDebugLine (Transformation|GetSocketLocation (Variables|Default|GetWeaponMesh) "Muzzle") (select _bblockinghit _impactpoint _traceend) "(R=1.000000,G=0.000000,B=0.000000,A=1.000000)" 0.1 2.0))
    (:then_1
      (Utilities|IsValid _returnvalue
        (:Is%20Valid
          (bind _asbp_hi_rs_character (Utilities|Casting|CastToBP_HiRS_Character _returnvalue))
          (Animation|PlayAnimMontage _asbp_hi_rs_character "/Game/HiRS/Character/Animations/Montages/AM_Shooting_Hip.AM_Shooting_Hip" 1.5 "None")
          (bind _asbp_hi_rs_character_2 (Utilities|Casting|CastToBP_HiRS_Character _hitactor))
          (Animation|PlayAnimMontage _asbp_hi_rs_character_2 (Utilities|Select :Index (Math|Random|RandomIntegerinRange 0 3) :Option%200 "/Game/HiRS/Character/Animations/Montages/OnHit/Hit_React_1_Montage.Hit_React_1_Montage" :Option%201 "/Game/HiRS/Character/Animations/Montages/OnHit/Hit_React_2_Montage.Hit_React_2_Montage" :Option%202 "/Game/HiRS/Character/Animations/Montages/OnHit/Hit_React_3_Montage.Hit_React_3_Montage" :Option%203 "/Game/HiRS/Character/Animations/Montages/OnHit/Hit_React_4_Montage.Hit_React_4_Montage") 1.0 "None"))))))

(event EventSetupShootingFunctionsforWeapon
  (if (Variables|Default|GetbWantToShoot)
    (switch Utilities|FlowControl|Switch|SwitchonEUsedWeapon (Variables|Default|GetCurrentUsedWeapon)
      (:primary
        (Class|HiRSWeapon|MomentalWeaponShot (Utilities|Struct|MakeMomentalWeaponData 0.1 0.15 10 25 true 5e+01 1e+04)))
      (:alternative
        (Class|HiRSWeapon|ProjectileWeaponShot (Utilities|Struct|MakeProjectileWeaponData 0.2 0.35 5 10 true "/Game/HiRS/Assets/Projectiles/BP_ExplosiveProjectile.BP_ExplosiveProjectile_C"))))))

(event EventSetupShootingFunctionsforSpecial
  (Class|HiRSWeapon|SpecialWeaponShot (Utilities|Struct|MakeProjectileWeaponData 1.0 1.0 10 40 false "/Game/HiRS/Assets/Projectiles/BP_GravityProjectile.BP_GravityProjectile_C")))

(event EventEventDrawShit
  (params (center :type Vector))
  (Utilities|FlowControl|FlipFlop
    (:A
      (Rendering|Debug|DrawDebugSphere center 2e+01 12 "(R=1.000000,G=0.000000,B=0.000000,A=1.000000)" 5.0 1.0))
    (:B
      (Rendering|Debug|DrawDebugSphere center 2e+01 12 "(R=0.000000,G=0.000000,B=1.000000,A=1.000000)" 5.0 1.0))))

(fn ConstructionScript)