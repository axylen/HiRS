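; Networked player character for HiRS with tackles, jetpack impulses and primary/alternative weapon switching.
; The server spawns and attaches the weapon, the local player gets the HUD, and construction tints the body materials.
; Tackles send montages through server and multicast events while crouching and lowering the camera arm by timeline.
; Death ragdolls the mesh with broken limb constraints, then the server triggers respawn and delayed cleanup; damage handling is an empty stub.
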(event Custom|OnDamage
  (params (Damage :type Float%20%28single-precision%29)))

(event Custom|MC_Montage
  (params (AnimMontage :type Anim%20Montage%20Object%20Reference))
  (Animation|PlayAnimMontage AnimMontage 1.0 "None"))

(event Custom|SpringArm_Tackle
  (params (Tackle :type Boolean))
  (if Tackle
    (bind _value (Timeline|SA_Tackle Play)
      (:Update
        (Transformation|SetRelativeLocation (Variables|Default|GetSpringArm) (Math|Vector|MakeVector 0.0 0.0 (Math|Float|Lerp 1.8e+02 9e+01 _value)) false false)
        (Variables|/Script/Engine.SpringArmComponent|SetTargetArmLength (Variables|Default|GetSpringArm) (Math|Float|Lerp 2e+02 1.5e+02 _value))))
    (else
      (Timeline|SA_Tackle Reverse))))

(event Custom|SetCharacterState
  (params (AnimMontage :type ECharacterState%20Enum))
  (Variables|Default|SetCharacterState AnimMontage))

(event Custom|Client_Respawn
  (bind _ashi_rs_pc (Utilities|Casting|CastToHiRS_PC (Game|GetPlayerController 0)))
  (Default|ServerSpawn _ashi_rs_pc))

(event Custom|ServerMontage
  (params (AnimMontage :type Anim%20Montage%20Object%20Reference))
  (CallFunction|MCMontage AnimMontage)
  (CallFunction|SwapTackleCollision true))

(event Custom|Server_JetpakJump
  (params (Target :type Character%20Movement%20Component%20Object%20Reference%20%28by%20ref%29) (Impulse :type Vector))
  (Physics|AddImpulse Target Impulse true))

(event Custom|MC_Death
  (Collision|SetCollisionEnabled (Variables|Default|GetCapsuleComponent) "NoCollision")
  (Physics|SetSimulatePhysics (Variables|Character|GetMesh) true)
  (CallFunction|BreakBones true true true true true))

(event EventOnTackle
  (CallFunction|SetCharacterState (Variables|Default|GetCharacterState))
  (CallFunction|ServerMontage (Utilities|Select :Index (Variables|Default|GetCharacterState) :idle 0 :move 0 :sprint 0 :TackleLT "/Game/HiRS/Character/Animations/AnimStarterPack/Tackle/AM_Tackle_Left.AM_Tackle_Left" :TackleFD "/Game/HiRS/Character/Animations/AnimStarterPack/Tackle/AM_Tackle.AM_Tackle" :TackleRT "/Game/HiRS/Character/Animations/AnimStarterPack/Tackle/AM_Tackle_Right.AM_Tackle_Right"))
  (CallFunction|SwapTackleCollision true))

(event Game|Damage|EventRadialDamage
  (params (DamageReceived :type Float%20%28single-precision%29) (DamageType :type Damage%20Type%20Object%20Reference) (Origin :type Vector :default "0, 0, 0") (HitInfo :type Hit%20Result%20Structure%20%28by%20ref%29) (InstigatedBy :type Controller%20Object%20Reference) (DamageCauser :type Actor%20Object%20Reference))
  (if (== (Utilities|GetClass DamageType) "/Game/HiRS/Assets/DamageTypes/ExplosiveDamage.ExplosiveDamage_C")
    (CallFunction|OnDamage DamageReceived)))

(event EventOnMovementModeChanged
  (params (PrevMovementMode :type EMovementMode%20Enum :default "MOVE_None") (NewMovementMode :type EMovementMode%20Enum :default "MOVE_None") (PrevCustomMode :type Byte :default 0) (NewCustomMode :type Byte :default 0))
  (Networking|SwitchHasAuthority
    (:Authority
      (if (Utilities|Enum|Equal(Enum) NewMovementMode "MOVE_Falling")
        (CallFunction|SwapTackleCollision false)))))

(event EventTick
  (params (DeltaSeconds :type Float%20%28single-precision%29))
  (|CallParentFunction DeltaSeconds))

(event EventEventonDeath
  (Utilities|FlowControl|Sequence
    (:then_0
      (Collision|SetCollisionEnabled (Variables|Default|GetCapsuleComponent) "NoCollision")
      (Physics|SetSimulatePhysics (Variables|Character|GetMesh) true)
      (CallFunction|BreakBones true true true true true))
    (:then_1
      (Networking|SwitchHasAuthority
        (:Authority
          (Utilities|FlowControl|Delay 1.0)
          (CallFunction|ClientRespawn)
          (Utilities|FlowControl|Delay 1e+01)
          (Actor|DestroyActor (Variables|Default|GetWeaponRef))
          (Actor|DestroyActor))))))

(event Game|Damage|EventPointDamage
  (params (Damage :type Float%20%28single-precision%29) (DamageType :type Damage%20Type%20Object%20Reference) (HitLocation :type Vector :default "0, 0, 0") (HitNormal :type Vector :default "0, 0, 0") (HitComponent :type Primitive%20Component%20Object%20Reference) (BoneName :type Name) (ShotFromDirection :type Vector) (InstigatedBy :type Controller%20Object%20Reference) (DamageCauser :type Actor%20Object%20Reference) (HitInfo :type Hit%20Result%20Structure%20%28by%20ref%29))
  (CallFunction|OnDamage Damage))

(event EventBeginPlay
  (|CallParentFunction)
  (Utilities|FlowControl|Sequence
    (:then_0
      (Networking|SwitchHasAuthority
        (:Authority
          (CallFunction|OnSpawn))
        (:Remote
          _))
      (if (Pawn|IsLocallyControlled)
        (bind _returnvalue (UserInterface|CreateWidget "/Game/HiRS/UMG/InGame/UMG_InGame.UMG_InGame_C" (Game|GetPlayerController 0)))
        (UserInterface|Viewport|AddtoPlayerScreen _returnvalue)))))

(event Input|ActionEvents|InputActionAlternativeFireOn
  (params (Key :type Key%20Structure :default "AnyKey"))
  (:Pressed
    (bind _weaponref (Variables|Default|GetWeaponRef)
      (:then
        (Class|HiRSWeapon|ChangeCurrentWeapon _weaponref "alternative"))
      (:else)))
  (:Released
    (bind _weaponref_2 (Variables|Default|GetWeaponRef)
      (:then
        (Class|HiRSWeapon|ChangeCurrentWeapon _weaponref_2 "primary"))
      (:else))))

(event Input|KeyboardEvents|G
  (params (Key :type Key%20Structure :default "AnyKey"))
  (:Pressed
    (Utilities|Time|SetGlobalTimeDilation 0.1))
  (:Released
    (Utilities|Time|SetGlobalTimeDilation 1.0)))

(fn ConstructionScript
  (Class|HiRSCharacter|SetBoneScale "1.000000,1.000000,1.000000" "1.000000,1.000000,1.000000" "1.000000,1.000000,1.000000" "1.000000,1.000000,1.000000" "1.000000,1.000000,1.000000" "1.000000,1.000000,1.000000" "1.000000,1.000000,1.000000")
  (CharacterSetting|SetupColor))

(fn OnSpawn
  (bind _self self)
  (bind _returnvalue (Game|SpawnActorfromClass "/Game/HiRS/Assets/Weapon/BP_Weapon.BP_Weapon_C" (Math|Transform|MakeTransform "0, 0, 0" "0, 0, 0" "1,1,1") "Undefined" _self _self))
  (bind _output_get (Variables|Default|SetWeaponRef _returnvalue))
  (Transformation|AttachComponentToComponent _output_get (Variables|Default|GetStaticMesh) "None" "KeepRelative" "KeepRelative" "KeepRelative" true))

(fn BreakBones
  (params (Spine :type Boolean) (leg_r :type Boolean) (leg_l :type Boolean) (arm_r :type Boolean) (arm_l :type Boolean))
  (LocalVariables|Set_Spine Spine)
  (LocalVariables|Set_Leg_r leg_r)
  (LocalVariables|Set_Leg_l leg_l)
  (LocalVariables|Set_Arm_r arm_r)
  (LocalVariables|Set_Arm_l arm_l)
  (Utilities|FlowControl|Sequence
    (:then_0
      (if (LocalVariables|Get_Spine)
        (Class|SkeletalMeshComponent|BreakConstraint (Variables|Character|GetMesh) "0,0.000000,0.000000" "0, 0, 0" "spine_01")))
    (:then_1
      (if (LocalVariables|Get_Leg_r)
        (Class|SkeletalMeshComponent|BreakConstraint (Variables|Character|GetMesh) "0,0.000000, 0" "0, 0, 0" "thigh_r")))
    (:then_2
      (if (LocalVariables|Get_Leg_l)
        (Class|SkeletalMeshComponent|BreakConstraint (Variables|Character|GetMesh) "0, 0, 0" "0.000000, 0, 0" "thigh_l")))
    (:then_3
      (if (LocalVariables|Get_Arm_r)
        (Class|SkeletalMeshComponent|BreakConstraint (Variables|Character|GetMesh) "0,0.000000, 0" "0.000000, 0, 0" "upperarm_r")))
    (:then_4
      (if (LocalVariables|Get_Arm_l)
        (Class|SkeletalMeshComponent|BreakConstraint (Variables|Character|GetMesh) "0,0.000000, 0" "0.000000, 0, 0" "upperarm_l")))))

(fn SwapTackleCollision
  (params (Tackle :type Boolean))
  (if Tackle
    (Character|Crouch)
    (Variables|Default|SetbIsTackle true)
    (CallFunction|SpringArmTackle true)
    (else
      (Character|UnCrouch)
      (Variables|Default|SetbIsTackle false)
      (CallFunction|SpringArmTackle false))))

(fn SetupColor
  (bind __color (LocalVariables|Get_Color))
  (bind __chestcolor (LocalVariables|Get_ChestColor))
  (bind _mesh (Variables|Character|GetMesh))
  (bind _mesh_2 (Variables|Character|GetMesh))
  (Utilities|FlowControl|Sequence
    (:then_0
      (bind _returnvalue (Rendering|Material|CreateDynamicMaterialInstance _mesh_2 0 0 :!class /Script/Engine.PrimitiveComponent))
      (Rendering|Material|SetVectorParameterValue _returnvalue "BodyColor" __color :!class /Script/Engine.MaterialInstanceDynamic)
      (bind _returnvalue_2 (Rendering|Material|CreateDynamicMaterialInstance _mesh 1 0 :!class /Script/Engine.PrimitiveComponent))
      (Rendering|Material|SetVectorParameterValue _returnvalue_2 "BodyColor" __chestcolor :!class /Script/Engine.MaterialInstanceDynamic))
    (:then_1
      (bind _returnvalue_3 (Rendering|Material|CreateDynamicMaterialInstance _mesh_2 2 0 :!class /Script/Engine.PrimitiveComponent))
      (Rendering|Material|SetVectorParameterValue _returnvalue_3 "BodyColor" __color :!class /Script/Engine.MaterialInstanceDynamic)
      (bind _returnvalue_4 (Rendering|Material|CreateDynamicMaterialInstance _mesh 3 0 :!class /Script/Engine.PrimitiveComponent))
      (Rendering|Material|SetVectorParameterValue _returnvalue_4 "BodyColor" __chestcolor :!class /Script/Engine.MaterialInstanceDynamic))))